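; BP_Shop is a shop tile actor whose door teleports the hero to a stored town position.
; Savepos stores that position in TownPos and applies the given rotation to the shop actor itself.
; When a HeroCharacter overlaps Door, it moves to TownPos with PlayerRot, keeping its scale, and the position is printed.
; BeginPlay zeroes SpawnPos, which this graph never reads, and PlayerRot is never assigned here.
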(event `self.ReceiveBeginPlay`
  (set `self.SpawnPos` (0.0 0.0 0.0)))

(event `self.Door.OnComponentBeginOverlap`
  (params (OverlappedComponent :type "PrimitiveComponent Object Reference") (OtherActor :type "Actor Object Reference") (OtherComp :type "PrimitiveComponent Object Reference") (OtherBodyIndex :type Integer) (bFromSweep :type Boolean) (SweepResult :type "HitResult Structure (by ref)"))
  (bind _townpos (`self.TownPos`))
  (bind _ashero_character (cast `HeroCharacter` OtherActor))
  (`self.K2_SetActorTransform` _ashero_character (`KismetMathLibrary.MakeTransform` _townpos (`self.PlayerRot`) (`self.GetActorScale3D` _ashero_character)) false false)
  (`KismetSystemLibrary.PrintString` (`KismetStringLibrary.Conv_VectorToString` _townpos)))

(fn `Savepos`
  (params (Pos :type "Vector Structure") (Rot :type "Rotator Structure"))
  (set `self.TownPos` Pos)
  (`self.K2_SetActorRotation` Rot))

(fn `UserConstructionScript`)