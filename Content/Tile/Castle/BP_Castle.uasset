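; BP_Castle is a castle tile actor that acts as a quest giver and spawns a guard NPC.
; On BeginPlay it picks a random row from the QuestData table and assigns it to its QuestGiverComponent.
; It then spawns the GuardNPC class at the Box component's location with the castle's rotation, ignoring collisions.
; InteractWith forwards to the QuestGiverComponent and returns its result.
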(event `self.ReceiveBeginPlay`
  (bind _outrownames (`DataTableFunctionLibrary.GetDataTableRowNames` "/Game/QuestSystem/QuestData.QuestData"))
  (set `/Game/QuestSystem/QuestGiverComponent.QuestData` (make `DataTableRowHandle` "/Game/QuestSystem/QuestData.QuestData" (`KismetArrayLibrary.Array_Random` _outrownames)) (`self.QuestGiverComponent`))
  (`|SpawnActorFromClass` "/Game/Characters/NPC/BP/GuardNPC.GuardNPC_C" (`KismetMathLibrary.MakeTransform` (`SceneComponent.K2_GetComponentLocation` (`self.Box`)) (`self.K2_GetActorRotation`)) "AlwaysSpawn" "OverrideRootScale" null null))

(fn `InteractWith`
  (returns (ObjectiveID :type String))
  (bind _objectiveid (`/Game/QuestSystem/IInteractionInterface.InteractWith` (`self.QuestGiverComponent`)))
  (return _objectiveid))

(fn `UserConstructionScript`)