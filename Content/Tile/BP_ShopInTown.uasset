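; BP_ShopInTown is a town shop entrance that teleports the hero to the level's BP_Shop.
; It finds that shop on BeginPlay and waits for a HeroCharacter to overlap its box.
; On overlap it sets the hero's special building code, saves a return spot just behind the hero with its own rotation on the shop, then moves the hero above the shop.
; A leftover debug print follows the teleport.
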(event `self.ReceiveBeginPlay`
  (bind _returnvalue (`GameplayStatics.GetActorOfClass` "/Game/Tile/BP_Shop.BP_Shop_C"))
  (set `self.MainShop` _returnvalue))

(event `self.Box.OnComponentBeginOverlap`
  (params (OverlappedComponent :type "PrimitiveComponent Object Reference") (OtherActor :type "Actor Object Reference") (OtherComp :type "PrimitiveComponent Object Reference") (OtherBodyIndex :type Integer) (bFromSweep :type Boolean) (SweepResult :type "HitResult Structure (by ref)"))
  (bind _mainshop (`self.MainShop`))
  (bind (_returnvalue_x _returnvalue_y _returnvalue_z) (`KismetMathLibrary.BreakVector` (`self.K2_GetActorLocation` _mainshop)))
  (bind _ashero_character (cast `HeroCharacter` OtherActor))
  (set `HeroCharacter.SpecialBuilingcode` 1 _ashero_character)
  (bind _returnvalue (+ (`self.K2_GetActorLocation` _ashero_character) (* (`self.GetActorForwardVector` _ashero_character) (-50.0 -50.0 0.0))))
  (`/Game/Tile/BP_Shop.Savepos` _mainshop _returnvalue (`self.K2_GetActorRotation`))
  (`self.K2_SetActorLocation` _ashero_character (`KismetMathLibrary.MakeVector` (+ _returnvalue_x 0.0) (+ _returnvalue_y 0.0) (+ _returnvalue_z 200.0)) false false)
  (`KismetSystemLibrary.PrintString` (`KismetStringLibrary.Conv_VectorToString` _returnvalue)))

(fn `UserConstructionScript`)