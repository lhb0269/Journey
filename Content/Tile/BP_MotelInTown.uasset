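; BP_MotelInTown is a motel tile actor that teleports the hero to the main motel.
; On BeginPlay it finds and caches the BP_Motel actor in the level.
; When a HeroCharacter overlaps its Box, it moves the hero to a point above that motel, using this actor's own rotation.
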(event `self.ReceiveBeginPlay`
  (bind _returnvalue (`GameplayStatics.GetActorOfClass` "/Game/Tile/BP_Motel.BP_Motel_C"))
  (set `self.MainMotel` _returnvalue))

(event `self.Box.OnComponentBeginOverlap`
  (params (OverlappedComponent :type "PrimitiveComponent Object Reference") (OtherActor :type "Actor Object Reference") (OtherComp :type "PrimitiveComponent Object Reference") (OtherBodyIndex :type Integer) (bFromSweep :type Boolean) (SweepResult :type "HitResult Structure (by ref)"))
  (bind (_returnvalue_x _returnvalue_y _returnvalue_z) (`KismetMathLibrary.BreakVector` (`self.K2_GetActorLocation` (`self.MainMotel`))))
  (bind _ashero_character (cast `HeroCharacter` OtherActor))
  (`self.K2_SetActorTransform` _ashero_character (`KismetMathLibrary.MakeTransform` (`KismetMathLibrary.MakeVector` (+ _returnvalue_x 0.0) (+ _returnvalue_y 0.0) (+ _returnvalue_z 200.0)) (`self.K2_GetActorRotation`)) false false))

(fn `UserConstructionScript`)