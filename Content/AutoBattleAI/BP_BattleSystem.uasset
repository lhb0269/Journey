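; BP_BattleSystem detects the end of an auto-battle and shows the matching result screen.
; While a battle is active, Tick polls the world for seven enemy classes, including goblins, orcs, golems and the final boss.
; Once none remain, it shows the battle widget, ends the battle and adds RewardGold to the hero.
; Final boss battles instead show the ending widget, without clearing the battle flag or awarding gold.
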(event `self.ReceiveTick`
  (params (DeltaSeconds :type "Float (single-precision)"))
  (if (`self.isBattleStart`)
    (bind _outactors (`GameplayStatics.GetAllActorsOfClass` "/Game/Monsters/MiddleBoss/Golem/BP_MBGolem.BP_MBGolem_C"))
    (if (== (`KismetArrayLibrary.Array_Length` _outactors) 0)
      (bind _outactors_2 (`GameplayStatics.GetAllActorsOfClass` "/Game/Monsters/Goblin/BP_Goblin.BP_Goblin_C"))
      (if (== (`KismetArrayLibrary.Array_Length` _outactors_2) 0)
        (bind _outactors_3 (`GameplayStatics.GetAllActorsOfClass` "/Game/Monsters/Orc/BP_Orc.BP_Orc_C"))
        (if (== (`KismetArrayLibrary.Array_Length` _outactors_3) 0)
          (bind _outactors_4 (`GameplayStatics.GetAllActorsOfClass` "/Game/Monsters/Golem/BP_Golem07.BP_Golem07_C"))
          (if (== (`KismetArrayLibrary.Array_Length` _outactors_4) 0)
            (bind _outactors_5 (`GameplayStatics.GetAllActorsOfClass` "/Game/Monsters/MiddleBoss/Goblin/BP_MBGoblin.BP_MBGoblin_C"))
            (if (== (`KismetArrayLibrary.Array_Length` _outactors_5) 0)
              (bind _outactors_6 (`GameplayStatics.GetAllActorsOfClass` "/Game/Monsters/MiddleBoss/Orc/BP_MBOrc.BP_MBOrc_C"))
              (if (== (`KismetArrayLibrary.Array_Length` _outactors_6) 0)
                (bind _outactors_7 (`GameplayStatics.GetAllActorsOfClass` "/Game/Monsters/FinalBoss/BP_FinalBoss.BP_FinalBoss_C"))
                (if (== (`KismetArrayLibrary.Array_Length` _outactors_7) 0)
                  (if (`self.isFinalBoss`)
                    (bind _returnvalue (`|CreateWidget` "/Game/UI/Widget/WBP_Ending.WBP_Ending_C" null (`self.RewardGold`)))
                    (`UserWidget.AddToViewport` _returnvalue 0)
                    (else
                      (bind _returnvalue_2 (`|CreateWidget` "/Game/UI/Widget/WBP_BattleSystem.WBP_BattleSystem_C" null (`self.RewardGold`)))
                      (`UserWidget.AddToViewport` _returnvalue_2 0)
                      (set `self.isBattleStart` false)
                      (bind _ashero_character (cast `HeroCharacter` (`GameplayStatics.GetPlayerCharacter` 0)))
                      (set `HeroCharacter.gold` (+ (`HeroCharacter.gold` _ashero_character) (`self.RewardGold`)) _ashero_character))))))))))))

(fn `UserConstructionScript`)