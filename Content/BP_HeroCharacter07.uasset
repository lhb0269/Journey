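; Player hero character for a town and ocean game, handling menus, NPC dialogue and world interaction.
; Adds the town map at start; keys open inventory, settings and quest log widgets.
; E messages overlapping shop, motel and partner NPCs, then line-traces from the camera for an interactable and broadcasts its objective ID.
; ToggleShip swaps body and ship visibility, while Tick polls click flags to show land-water transition widgets.
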(event `self.ReceiveBeginPlay`
  (bind _returnvalue (`|CreateWidget` "/Game/UI/Widget/WBP_TownMapUI.WBP_TownMapUI_C"))
  (`UserWidget.AddToViewport` _returnvalue 0))

(event `Key|Tab`
  (params (Key :type "Key Structure"))
  (bind _returnvalue (`GameplayStatics.GetPlayerController` 0))
  (:`Pressed`
    (`GameplayStatics.PlaySound2D` "/Game/UI/Sound/Effect/click.click" 1.0 1.0 0.0 null null)
    (bind _returnvalue_2 (`|CreateWidget` "/Game/UI/Widget/InventoryShop/WBP_Inventory.WBP_Inventory_C" (`GameplayStatics.GetPlayerController` 0)))
    (`UserWidget.AddToViewport` _returnvalue_2 0)
    (set `PlayerController.bShowMouseCursor` true _returnvalue)
    (`WidgetBlueprintLibrary.SetInputMode_UIOnlyEx` _returnvalue _returnvalue_2)))

(event `Key|E`
  (params (Key :type "Key Structure"))
  (:`Pressed`
    (`|ExecutionSequence`
      (:`then_0`
        (for _array_element (`self.GetOverlappingActors` "/Game/Characters/NPC/BP/ShopNPC.ShopNPC_C")
          (if (`KismetSystemLibrary.DoesImplementInterface` _array_element "/Game/Characters/NPC/BP/BP_Dialog.BP_Dialog_C")
            (message `/Game/Characters/NPC/BP/BP_Dialog.Talk` _array_element (`self.SpecialBuilingcode`)))))
      (:`then_1`
        (for _array_element_2 (`self.GetOverlappingActors` "/Game/Characters/NPC/BP/MotelNPC.MotelNPC_C")
          (if (`KismetSystemLibrary.DoesImplementInterface` _array_element_2 "/Game/Characters/NPC/BP/BP_Dialog.BP_Dialog_C")
            (message `/Game/Characters/NPC/BP/BP_Dialog.Talk` _array_element_2 (`self.SpecialBuilingcode`)))))
      (:`then_2`
        (for _array_element_3 (`self.GetOverlappingActors` "/Game/Characters/NPC/BP/PartnerNPC.PartnerNPC_C")
          (if (`KismetSystemLibrary.DoesImplementInterface` _array_element_3 "/Game/Characters/NPC/BP/BP_Dialog.BP_Dialog_C")
            (message `/Game/Characters/NPC/BP/BP_Dialog.Talk` _array_element_3 (`self.SpecialBuilingcode`)))))
      (:`then_3`
        (`self.InteractionTrace`)
        (bind _lookatactor (`self.LookAtActor`)
          (:`then`
            (bind _objectiveid (message `/Game/QuestSystem/IInteractionInterface.InteractWith` _lookatactor))
            (`self.OnObjectiveIDCalled` _objectiveid))
          (:`else`))))))

(event `Key|P`
  (params (Key :type "Key Structure"))
  (bind _returnvalue (`GameplayStatics.GetPlayerController` 0))
  (:`Pressed`
    (`GameplayStatics.PlaySound2D` "/Game/UI/Sound/Effect/click.click" 1.0 1.0 0.0 null null)
    (bind _returnvalue_2 (`|CreateWidget` "/Game/UI/Widget/WBP_Setting.WBP_Setting_C" (`GameplayStatics.GetPlayerController` 0)))
    (`UserWidget.AddToViewport` _returnvalue_2 0)
    (set `PlayerController.bShowMouseCursor` true _returnvalue)
    (`WidgetBlueprintLibrary.SetInputMode_UIOnlyEx` _returnvalue null)))

(event `Key|J`
  (params (Key :type "Key Structure"))
  (:`Pressed`
    (bind _returnvalue (`|CreateWidget` "/Game/QuestSystem/UI/WBP_QuestLog.WBP_QuestLog_C"))
    (`UserWidget.AddToViewport` _returnvalue 0)))

(event `ToggleShip`
  (`/Engine/EditorBlueprintResources/StandardMacros.FlipFlop`
    (:`A`
      (`SceneComponent.SetVisibility` (`self.Ship`) true false)
      (`SceneComponent.SetVisibility` (`self.Vest`) false false)
      (`SceneComponent.SetVisibility` (`self.Mesh`) false false))
    (:`B`
      (`SceneComponent.SetVisibility` (`self.Ship`) false false)
      (`SceneComponent.SetVisibility` (`self.Vest`) true false)
      (`SceneComponent.SetVisibility` (`self.Mesh`) true false))))

(event `self.ReceiveTick`
  (params (DeltaSeconds :type "Float (single-precision)"))
  (`|ExecutionSequence`
    (:`then_0`
      (if (`self.landClick`)
        (bind _returnvalue (`|CreateWidget` "/Game/UI/Widget/WBP_WaterToLand.WBP_WaterToLand_C" (`GameplayStatics.GetPlayerController` 0)))
        (`UserWidget.AddToViewport` _returnvalue 0)
        (set `self.landClick` false)))
    (:`then_1`
      (if (`self.oceanClick`)
        (bind _returnvalue_2 (`|CreateWidget` "/Game/UI/Widget/WBP_LandToWater.WBP_LandToWater_C" (`GameplayStatics.GetPlayerController` 0)))
        (`UserWidget.AddToViewport` _returnvalue_2 0)
        (set `self.oceanClick` false)))))

(fn `InteractionTrace`
  (bind _returnvalue (`GameplayStatics.GetPlayerCameraManager` 0))
  (bind _returnvalue_2 (`self.K2_GetActorLocation` _returnvalue))
  (bind (_outhit _returnvalue_3) (`KismetSystemLibrary.LineTraceSingle` _returnvalue_2 (+ _returnvalue_2 (* (`self.GetActorForwardVector` _returnvalue) 200.0)) "TraceTypeQuery2"))
  (if _returnvalue_3
    (bind (_bblockinghit _binitialoverlap _time _distance _location _impactpoint _normal _impactnormal _physmat _hitactor) (`GameplayStatics.BreakHitResult` _outhit))
    (if (`KismetSystemLibrary.DoesImplementInterface` _hitactor "/Game/QuestSystem/IInteractionInterface.IInteractionInterface_C")
      (bind _output_get (set `self.LookAtActor` _hitactor))
      (message `/Game/QuestSystem/IInteractionInterface.LookAt` _output_get)
      (else
        (set `self.LookAtActor` null)))
    (else
      (set `self.LookAtActor` null))))

(fn `UserConstructionScript`)