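; Goblin enemy that hunts hero units and reports an objective ID to the player's hero when killed.
; A custom event starts it toward the nearest "HeroUnit" with AIMoveTo; Tick searches "Unit" actors whenever the target is invalid.
; Reaching or holding a target sets the attack flag, though the ApplyDamage logic is unconnected.
; AnyDamage updates damage and health widgets, then sets death or hit-reaction flags that interrupt attacking.
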(event `CustomEvent`
  (bind _targethero (`self.TargetHero`))
  (set `self.isStart` true)
  ;[1 1 1] Search BaseUnit
  (bind _outactors (`GameplayStatics.GetAllActorsWithTag` "HeroUnit"))
  (for _array_element _outactors
    (bind _returnvalue (`self.GetDistanceTo` _array_element))
    (if (< _returnvalue (`self.Distatnce`))
      (set `self.TargetHero` _array_element)
      (set `self.Distatnce` _returnvalue)))
  (`|AIMoveTo` self (`self.K2_GetActorLocation` _targethero) _targethero 200.0
    (:`OnSuccess`
      (set `self.IsAttack` true))))

(event `self.ReceiveTick`
  (params (DeltaSeconds :type "Float (single-precision)"))
  (bind _targethero (`self.TargetHero`))
  (if (`self.isStart`)
    (`/Engine/EditorBlueprintResources/StandardMacros.IsValid` (`self.TargetHero`)
      (:`Is Valid`
        (set `self.IsAttack` true))
      (:`Is Not Valid`
        ;[1 1 1] Search BaseUnit
        (bind _outactors (`GameplayStatics.GetAllActorsWithTag` "Unit"))
        (for _array_element _outactors
          (bind _returnvalue (`self.GetDistanceTo` _array_element))
          (if (< _returnvalue (`self.Distatnce`))
            (set `self.TargetHero` _array_element)
            (set `self.Distatnce` _returnvalue)))
        (`|AIMoveTo` self (`self.K2_GetActorLocation` _targethero) _targethero 200.0
          (:`OnSuccess`
            (set `self.isAttack` true)))))))

(event `self.ReceiveAnyDamage`
  (params (Damage :type "Float (single-precision)") (DamageType :type "DamageType Object Reference") (InstigatedBy :type "Controller Object Reference") (DamageCauser :type "Actor Object Reference"))
  (bind _hp (`self.HP`))
  ;[1 1 1] Attacked
  (if (not (`self.isAttacked`))
    (bind _aswbp_damage (cast `/Game/UI/Widget/WBP_Damage` (`WidgetComponent.GetWidget` (`self.Damage`))))
    (`/Game/UI/Widget/WBP_Damage.ApplyDamage` _aswbp_damage (`KismetTextLibrary.Conv_DoubleToText` Damage "HalfToEven"))
    (bind _output_get (set `self.HP` (- _hp Damage)))
    (bind _ashealth_bar (cast `/Game/AutoBattleAI/HealthBar` (`WidgetComponent.GetUserWidgetObject` (`self.hpbar`))))
    (set `/Game/AutoBattleAI/HealthBar.HP` _output_get _ashealth_bar)
    (if (<= _hp 0.0)
      (set `self.isDead` true)
      (set `self.isAttack` false)
      (bind _asbp_hero_character (cast `/Game/UI/CharacterUI/BP_HeroCharacter` (`GameplayStatics.GetPlayerCharacter` 0)))
      (`/Game/UI/CharacterUI/BP_HeroCharacter.OnObjectiveIDCalled` _asbp_hero_character (`self.ObjectiveID`))
      (else
        (set `self.ArmorCount` (+ (`self.ArmorCount`) 1))
        (if (> (`self.ArmorCount`) 0)
          (set `self.ArmorCount` 0)
          (if (not (`self.isAttacked`))
            (set `self.isAttacked` true)
            (set `self.isAttack` false)))))))

(fn `UserConstructionScript`)