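; Final boss monster that fights actors tagged HeroUnit and notifies the player's objective when killed.
; After StartBattle, it chases the nearest hero, faces it, and sets attack or random skill flags depending on MP.
; Meteor, Laser and EarthAttack events deliver overhead meteor spawns, target damage and close-range area damage.
; Damage updates widgets, and an armor hit counter periodically sets IsAttacked, halting attacks and ignoring damage while set.
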(event `self.ReceiveBeginPlay`
  (bind _ashealth_bar (cast `/Game/AutoBattleAI/HealthBar` (`WidgetComponent.GetUserWidgetObject` (`self.hpbar`))))
  (set `/Game/AutoBattleAI/HealthBar.MAXHP` (`self.HP`) _ashealth_bar))

(event `StartBattle`
  (bind _targethero (`self.TargetHero`))
  (set `self.isStart` true)
  ;[1 1 1] Search BaseUnit
  (bind _outactors (`GameplayStatics.GetAllActorsWithTag` "HeroUnit"))
  (for _array_element _outactors
    (bind _returnvalue (`self.GetDistanceTo` _array_element))
    (if (< _returnvalue (`self.Distatnce`))
      (set `self.TargetHero` _array_element)
      (set `self.Distatnce` _returnvalue)))
  (`|AIMoveTo` self (`self.K2_GetActorLocation` _targethero) _targethero 200.0
    (:`OnSuccess`
      (set `self.IsAttack` true))))

(event `self.ReceiveTick`
  (params (DeltaSeconds :type "Float (single-precision)"))
  (bind _returnvalue (`KismetMathLibrary.RandomIntegerInRange` 0 2))
  (bind _targethero (`self.TargetHero`))
  (if (`self.isDead`)
    _
    (elif (`self.isStart`)
      (`/Engine/EditorBlueprintResources/StandardMacros.IsValid` (`self.TargetHero`)
        (:`Is Valid`
          ;[1 1 1] Search BaseUnit
          (`self.K2_SetActorRotation` (`KismetMathLibrary.FindLookAtRotation` (`self.K2_GetActorLocation`) (`self.K2_GetActorLocation` (`self.TargetHero`))))
          (if (>= (`self.MP`) 20.0)
            (if (== _returnvalue 0)
              (set `self.isSkill1` true)
              (set `self.MP` 0.0)
              (elif (== _returnvalue 1)
                (set `self.isSkill2` true)
                (set `self.MP` 0.0)
                (elif true
                  (set `self.isSkill3` true)
                  (set `self.MP` 0.0))))
            (else
              (set `self.IsAttack` true))))
        (:`Is Not Valid`
          ;[1 1 1] Search BaseUnit
          (set `self.Distatnce` 1000000.0)
          (bind _outactors (`GameplayStatics.GetAllActorsWithTag` "HeroUnit"))
          (for _array_element _outactors
            (bind _returnvalue_2 (`self.GetDistanceTo` _array_element))
            (if (< _returnvalue_2 (`self.Distatnce`))
              (set `self.TargetHero` _array_element)
              (set `self.Distatnce` _returnvalue_2)))
          (`|AIMoveTo` self (`self.K2_GetActorLocation` _targethero) _targethero 200.0
            (:`OnSuccess`
              (set `self.isAttack` true))))))))

(event `self.ReceiveAnyDamage`
  (params (Damage :type "Float (single-precision)") (DamageType :type "DamageType Object Reference") (InstigatedBy :type "Controller Object Reference") (DamageCauser :type "Actor Object Reference"))
  (bind _hp (`self.HP`))
  ;[1 1 1] Attacked
  (if (not (`self.isAttacked`))
    (bind _aswbp_damage (cast `/Game/UI/Widget/WBP_Damage` (`WidgetComponent.GetWidget` (`self.Damage`))))
    (`/Game/UI/Widget/WBP_Damage.ApplyDamage` _aswbp_damage (`KismetTextLibrary.Conv_DoubleToText` Damage "HalfToEven"))
    (bind _output_get (set `self.HP` (- _hp Damage)))
    (bind _ashealth_bar (cast `/Game/AutoBattleAI/HealthBar` (`WidgetComponent.GetUserWidgetObject` (`self.hpbar`))))
    (set `/Game/AutoBattleAI/HealthBar.HP` _output_get _ashealth_bar)
    (if (<= _hp 0.0)
      (set `self.isDead` true)
      (set `self.isAttack` false)
      (bind _asbp_hero_character (cast `/Game/UI/CharacterUI/BP_HeroCharacter` (`GameplayStatics.GetPlayerCharacter` 0)))
      (`/Game/UI/CharacterUI/BP_HeroCharacter.OnObjectiveIDCalled` _asbp_hero_character (`self.ObjectiveID`))
      (else
        (set `self.ArmorCount` (+ (`self.ArmorCount`) 1))
        (if (> (`self.ArmorCount`) 20)
          (set `self.ArmorCount` 0)
          (if (not (`self.isAttacked`))
            (set `self.isAttacked` true)
            (set `self.isAttack` false)))))))

(event `Meteor`
  (bind _outactors (`GameplayStatics.GetAllActorsWithTag` "HeroUnit"))
  (for _array_element _outactors
    (bind (_returnvalue_x _returnvalue_y _returnvalue_z) (`KismetMathLibrary.BreakVector` (`self.K2_GetActorLocation` _array_element)))
    (`|SpawnActorFromClass` "/Game/Effect/Meteo/BP_meteo.BP_meteo_C" (`KismetMathLibrary.Conv_VectorToTransform` (`KismetMathLibrary.MakeVector` _returnvalue_x _returnvalue_y (+ _returnvalue_z 3000.0))) "Undefined" "OverrideRootScale" _array_element null)))

(event `Laser`
  (`GameplayStatics.ApplyDamage` (`self.TargetHero`) (`self.Power`)))

(event `EarthAttack`
  (bind _outactors (`GameplayStatics.GetAllActorsWithTag` "HeroUnit"))
  (for _array_element _outactors
    (if (< (`self.GetDistanceTo` _array_element) 400.0)
      (`GameplayStatics.ApplyDamage` _array_element 10.0))))

(fn `UserConstructionScript`)