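; BP_TileInfo is a tile actor in the AI folder that tracks and shows mouse-cursor hover.
; Cursor-over events on the Floor component set IsOver and swap its material between a highlight reference and the base tile material.
; On BeginPlay, a tile flagged IsHere gives its Area component the field volume preview material.
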(event `self.ReceiveBeginPlay`
  (if (`self.IsHere`)
    (`PrimitiveComponent.SetMaterial` (`self.Area`) 0 "/Engine/EditorResources/FieldNodes/_Resources/M_FieldVolumePreview.M_FieldVolumePreview")))

(event `self.Floor.OnBeginCursorOver`
  (params (TouchedComponent :type "PrimitiveComponent Object Reference"))
  (set `self.IsOver` true)
  (`PrimitiveComponent.SetMaterial` (`self.Floor`) 0 "/DatasmithContent/Materials/AliasReference.AliasReference"))

(event `self.Floor.OnEndCursorOver`
  (params (TouchedComponent :type "PrimitiveComponent Object Reference"))
  (set `self.IsOver` false)
  (`PrimitiveComponent.SetMaterial` (`self.Floor`) 0 "/Game/AI/BTileMaterial.BTileMaterial"))

(fn `UserConstructionScript`)