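; BP_Player is a placeable unit for a tile-based auto-battle against BP_Monster actors.
; Clicking its cube reveals tile areas with HeightNum under 3, and ClickEnd moves it onto the hovered unoccupied tile.
; StartBattle picks the nearest living monster within Distance and uses AIMoveTo, enabling attack on arrival.
; Capsule overlaps then deal Power damage; incoming damage lowers HP, but the death branch assigns IsDead to itself.
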(event `self.ReceiveBeginPlay`
  (set `self.StartLocation` (`SceneComponent.K2_GetComponentLocation` (`self.CapsuleComponent`))))

(event `self.ReceiveTick`
  (params (DeltaSeconds :type "Float (single-precision)")))

(event `StartBattle`
  (bind _targetmonster (`self.TargetMonster`))
  (set `self.IsStart` true)
  (if (`self.IsStart`)
    (bind _outactors (`GameplayStatics.GetAllActorsOfClass` "/Game/AI/AI_Ver1/BP_Monster.BP_Monster_C"))
    (for _array_element _outactors
      (if (not (`/Game/AI/AI_Ver1/BP_Monster.isDead` _array_element))
        (bind _returnvalue (`self.GetDistanceTo` _array_element))
        (if (< _returnvalue (`self.Distance`))
          (set `self.TargetMonster` _array_element)
          (set `self.Distance` _returnvalue))))
    (`|AIMoveTo` self (`self.K2_GetActorLocation` _targetmonster) _targetmonster
      (:`OnSuccess`
        (set `self.IsAttack` true)))))

(event `self.Cube.OnClicked`
  (params (TouchedComponent :type "PrimitiveComponent Object Reference") (ButtonPressed :type "Key Structure"))
  (set `self.IsClick` true)
  (bind _outactors (`GameplayStatics.GetAllActorsOfClass` "/Game/AI/BP_TileInfo.BP_TileInfo_C"))
  (for _array_element _outactors
    (if (> 3 (`TileInfo.heightNum` _array_element))
      (`SceneComponent.SetVisibility` (`/Game/AI/BP_TileInfo.Area` _array_element) true false))))

(event `ClickEnd`
  (if (`self.IsClick`)
    (set `self.IsClick` false)
    (bind _outactors (`GameplayStatics.GetAllActorsOfClass` "/Game/AI/BP_TileInfo.BP_TileInfo_C"))
    (for _array_element _outactors
      (bind _area (`/Game/AI/BP_TileInfo.Area` _array_element))
      (`SceneComponent.SetVisibility` _area false false)
      (if (`/Game/AI/BP_TileInfo.IsOver` _array_element)
        (if (not (`/Game/AI/BP_TileInfo.IsHere` _array_element))
          (bind (_returnvalue_x _returnvalue_y _returnvalue_z) (`KismetMathLibrary.BreakVector` (`SceneComponent.K2_GetComponentLocation` _area)))
          (`SceneComponent.K2_SetWorldLocation` (`self.CapsuleComponent`) (`KismetMathLibrary.MakeVector` _returnvalue_x _returnvalue_y (+ _returnvalue_z 100.0)) false false))))))

(event `self.CapsuleComponent.OnComponentBeginOverlap`
  (params (OverlappedComponent :type "PrimitiveComponent Object Reference") (OtherActor :type "Actor Object Reference") (OtherComp :type "PrimitiveComponent Object Reference") (OtherBodyIndex :type Integer) (bFromSweep :type Boolean) (SweepResult :type "HitResult Structure (by ref)"))
  (if (`self.IsAttack`)
    (`GameplayStatics.ApplyDamage` OtherActor (`self.Power`) null self)))

(event `self.ReceiveAnyDamage`
  (params (Damage :type "Float (single-precision)") (DamageType :type "DamageType Object Reference") (InstigatedBy :type "Controller Object Reference") (DamageCauser :type "Actor Object Reference"))
  (bind _hp (`self.HP`))
  (set `self.HP` (- _hp Damage))
  (if (<= _hp 0.0)
    (set `self.isDead` (`self.isDead`))))

(fn `UserConstructionScript`)