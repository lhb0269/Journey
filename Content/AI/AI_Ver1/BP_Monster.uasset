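; BP_Monster is an enemy that damages non-monster actors overlapping its capsule while IsAttack is set.
; StartBattle only gathers BP_Hero actors; the nearest-hero targeting and AIMoveTo chain that sets IsAttack is disconnected.
; AnyDamage shows damage through WBP_Damage and updates HP and the health bar.
; At zero HP it spawns a death effect, reports its ObjectiveID to the player's hero character, drops BP_Gold and destroys itself.
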(event `self.ReceiveBeginPlay`)

(event `self.ReceiveTick`
  (params (DeltaSeconds :type "Float (single-precision)")))

(event `StartBattle`
  (set `self.isStart` true)
  (if (`self.isStart`)
    (bind _outactors (`GameplayStatics.GetAllActorsOfClass` "/Game/AI/AI_Ver2/BP_Hero.BP_Hero_C"))))

(event `self.ReceiveAnyDamage`
  (params (Damage :type "Float (single-precision)") (DamageType :type "DamageType Object Reference") (InstigatedBy :type "Controller Object Reference") (DamageCauser :type "Actor Object Reference"))
  (bind _hp (`self.HP`))
  (bind _aswbp_damage (cast `/Game/UI/Widget/WBP_Damage` (`WidgetComponent.GetWidget` (`self.Damage`))))
  (`/Game/UI/Widget/WBP_Damage.ApplyDamage` _aswbp_damage (`KismetTextLibrary.Conv_DoubleToText` Damage "HalfToEven"))
  (bind _output_get (set `self.HP` (- _hp Damage)))
  (bind _ashealth_bar (cast `/Game/AutoBattleAI/HealthBar` (`WidgetComponent.GetUserWidgetObject` (`self.hpbar`))))
  (set `/Game/AutoBattleAI/HealthBar.HP` _output_get _ashealth_bar)
  (if (<= _hp 0.0)
    (set `self.isDead` (`self.isDead`))
    (`NiagaraFunctionLibrary.SpawnSystemAtLocation` "/Game/Texture/Particle/NS_Death.NS_Death" (`self.K2_GetActorLocation`))
    (bind _asbp_hero_character (cast `/Game/UI/CharacterUI/BP_HeroCharacter` (`GameplayStatics.GetPlayerCharacter` 0)))
    (`/Game/UI/CharacterUI/BP_HeroCharacter.OnObjectiveIDCalled` _asbp_hero_character (`self.ObjectiveID`))
    (`|SpawnActorFromClass` "/Game/Items/BP_Gold.BP_Gold_C" (`KismetMathLibrary.Conv_VectorToTransform` (`self.K2_GetActorLocation`)) "Undefined" "OverrideRootScale" null null)
    (`self.K2_DestroyActor`)))

(event `self.Capsule.OnComponentBeginOverlap`
  (params (OverlappedComponent :type "PrimitiveComponent Object Reference") (OtherActor :type "Actor Object Reference") (OtherComp :type "PrimitiveComponent Object Reference") (OtherBodyIndex :type Integer) (bFromSweep :type Boolean) (SweepResult :type "HitResult Structure (by ref)"))
  (cast `/Game/AI/AI_Ver1/BP_Monster` OtherActor
    (:`CastFailed`
      (if (`self.isAttack`)
        (`GameplayStatics.ApplyDamage` OtherActor (`self.Power`) null self)))))

(fn `UserConstructionScript`)