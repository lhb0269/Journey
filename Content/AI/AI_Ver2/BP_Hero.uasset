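; BP_Hero is an auto-battling hero that, once StartBattle runs, moves to the nearest living BP_Monster and flags itself as attacking.
; Tick searches for a new target when the current one becomes invalid.
; Attacks and capsule overlaps build MP, with overlaps also dealing Power damage; full MP on Tick resets it, flags Skill1 and spawns a steam effect.
; BeginPlay binds the HP/MP bar widget to the hero.
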(event `self.ReceiveBeginPlay`
  (bind _aswbp_unit_hpbar (cast `/Game/UI/Widget/WBP_UnitHPBar` (`WidgetComponent.GetUserWidgetObject` (`self.HPMPBar`))))
  (set `/Game/UI/Widget/WBP_UnitHPBar.Unit` self _aswbp_unit_hpbar))

(event `StartBattle`
  (set `self.IsStart` true)
  (if (`self.IsStart`)
    (bind _outactors (`GameplayStatics.GetAllActorsOfClass` "/Game/AI/AI_Ver1/BP_Monster.BP_Monster_C"))
    (for _array_element _outactors
      (if (not (`/Game/AI/AI_Ver1/BP_Monster.isDead` _array_element))
        (bind _returnvalue (`self.GetDistanceTo` _array_element))
        (if (< _returnvalue (`self.distance`))
          (set `self.Target Monster` _array_element)
          (set `self.distance` _returnvalue))))
    (`|AIMoveTo` self (0.0 0.0 0.0) (`self.Target Monster`) 80.0
      (:`OnSuccess`
        (set `self.IsAttack` true)))))

(event `self.ReceiveTick`
  (params (DeltaSeconds :type "Float (single-precision)"))
  (bind _target_monster (`self.Target Monster`))
  (if (`self.IsStart`)
    (`/Engine/EditorBlueprintResources/StandardMacros.IsValid` (`self.Target Monster`)
      (:`Is Valid`
        (if (>= (`self.nowMP`) (`self.maxMP`))
          (set `self.nowMP` 0.0)
          (set `self.isSkill1` true)
          (`GameplayStatics.SpawnEmitterAtLocation` "/Game/StarterContent/Particles/P_Steam_Lit.P_Steam_Lit" (`self.K2_GetActorLocation`))
          (elif (not (`self.isAttack`))
            (set `self.isAttack` true)
            (set `self.nowMP` (+ (`self.nowMP`) 10.0)))))
      (:`Is Not Valid`
        (set `self.IsAttack` false)
        (set `self.distance` 10000.0)
        (bind _outactors (`GameplayStatics.GetAllActorsOfClass` "/Game/AI/AI_Ver1/BP_Monster.BP_Monster_C"))
        (if (> (`KismetArrayLibrary.Array_Length` _outactors) 0)
          (for _array_element _outactors
            (if (not (`/Game/AI/AI_Ver1/BP_Monster.isDead` _array_element))
              (bind _returnvalue (`self.GetDistanceTo` _array_element))
              (if (< _returnvalue (`self.distance`))
                (set `self.Target Monster` _array_element)
                (set `self.distance` _returnvalue))))
          (`|AIMoveTo` self (`self.K2_GetActorLocation` _target_monster) _target_monster 80.0
            (:`OnSuccess`
              (set `self.IsAttack` true)
              (set `self.nowMP` (+ (`self.nowMP`) 10.0)))))))))

(event `self.Capsule.OnComponentBeginOverlap`
  (params (OverlappedComponent :type "PrimitiveComponent Object Reference") (OtherActor :type "Actor Object Reference") (OtherComp :type "PrimitiveComponent Object Reference") (OtherBodyIndex :type Integer) (bFromSweep :type Boolean) (SweepResult :type "HitResult Structure (by ref)"))
  (bind _nowmp (`self.nowMP`))
  (`GameplayStatics.ApplyDamage` OtherActor (`self.power`) null self)
  (set `self.nowMP` (+ _nowmp 5.0))
  (if (>= _nowmp 100.0)
    (set `self.nowMP` 0.0)))

(fn `UserConstructionScript`)