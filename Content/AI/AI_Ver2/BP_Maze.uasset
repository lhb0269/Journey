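; BP_Maze is a ranged auto-battle AI unit that, once battle starts, hunts the nearest actor tagged Monster07.
; Tick retargets when the target becomes invalid, builds MP as attacks trigger, and at full MP flags Skill1 with a steam effect.
; ThrowFireBall turns to the target and spawns a fireball from an arrow component.
; Damage reduces HP and sets hit or death state flags; a widget bar is bound to the unit.
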(event `StartBattle`
  (set `self.IsStart` true)
  (if (`self.IsStart`)
    (bind _outactors (`GameplayStatics.GetAllActorsWithTag` "Monster07"))
    (for _array_element _outactors
      (bind _returnvalue (`self.GetDistanceTo` _array_element))
      (if (< _returnvalue (`self.distance`))
        (set `self.Target Monster` _array_element)
        (set `self.distance` _returnvalue)))
    (`|AIMoveTo` self (0.0 0.0 0.0) (`self.Target Monster`) 800.0
      (:`OnSuccess`
        (set `self.IsAttack` true)))))

(event `self.ReceiveBeginPlay`
  (bind _aswbp_unit_hpbar (cast `/Game/UI/Widget/WBP_UnitHPBar` (`WidgetComponent.GetUserWidgetObject` (`self.HPMPBar`))))
  (set `/Game/UI/Widget/WBP_UnitHPBar.Unit` self _aswbp_unit_hpbar))

(event `self.ReceiveTick`
  (params (DeltaSeconds :type "Float (single-precision)"))
  (bind _target_monster (`self.Target Monster`))
  (if (`self.IsStart`)
    (`/Engine/EditorBlueprintResources/StandardMacros.IsValid` (`self.Target Monster`)
      (:`Is Valid`
        (if (>= (`self.nowMP`) (`self.maxMP`))
          (set `self.nowMP` 0.0)
          (set `self.isSkill1` true)
          (`GameplayStatics.SpawnEmitterAtLocation` "/Game/StarterContent/Particles/P_Steam_Lit.P_Steam_Lit" (`self.K2_GetActorLocation`))
          (elif (not (`self.isAttack`))
            (set `self.isAttack` true)
            (set `self.nowMP` (+ (`self.nowMP`) 10.0)))))
      (:`Is Not Valid`
        (set `self.IsAttack` false)
        (set `self.distance` 10000.0)
        (bind _outactors (`GameplayStatics.GetAllActorsWithTag` "Monster07"))
        (if (> (`KismetArrayLibrary.Array_Length` _outactors) 0)
          (for _array_element _outactors
            (bind _returnvalue (`self.GetDistanceTo` _array_element))
            (if (< _returnvalue (`self.distance`))
              (set `self.Target Monster` _array_element)
              (set `self.distance` _returnvalue)))
          (`|AIMoveTo` self (`self.K2_GetActorLocation` _target_monster) _target_monster 800.0
            (:`OnSuccess`
              (set `self.IsAttack` true)
              (set `self.nowMP` (+ (`self.nowMP`) 10.0)))))))))

(event `ThrowFireBall`
  (`self.K2_SetActorRotation` (`KismetMathLibrary.FindLookAtRotation` (`self.K2_GetActorLocation`) (`self.K2_GetActorLocation` (`self.Target Monster`))))
  (`|SpawnActorFromClass` "/Game/AI/AI_Ver2/BP_FireBall.BP_FireBall_C" (`SceneComponent.K2_GetComponentToWorld` (`self.Arrow1`)) "Undefined" "OverrideRootScale" null null))

(event `self.ReceiveAnyDamage`
  (params (Damage :type "Float (single-precision)") (DamageType :type "DamageType Object Reference") (InstigatedBy :type "Controller Object Reference") (DamageCauser :type "Actor Object Reference"))
  (bind _returnvalue (- (`self.nowHP`) Damage))
  ;[1 1 1] Attacked
  (if (not (`self.isAttacked`))
    (set `self.nowHP` _returnvalue)
    (if (<= _returnvalue 0.0)
      (set `self.isDeath` true)
      (set `self.isAttack` false)
      (set `self.isSkill1` false)
      (set `self.isAttacked` true)
      (else
        (set `self.isAttacked` true)
        (set `self.isAttack` false)
        (set `self.isSkill1` false)))))

(fn `UserConstructionScript`)