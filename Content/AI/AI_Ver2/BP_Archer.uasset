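; BP_Archer is an auto-battling ranged unit that hunts BP_Monster actors.
; StartBattle picks the nearest living monster and uses AIMoveTo to close to firing range, then sets IsAttack.
; Tick searches again whenever the target becomes invalid, while ShotArrow faces the target and spawns a BP_Arrow aimed at it.
; A damage and MP-gain chain remains in the graph but is unconnected.
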(event `StartBattle`
  (bind _target_monster (`self.Target Monster`))
  (set `self.IsStart` true)
  (if (`self.IsStart`)
    (bind _outactors (`GameplayStatics.GetAllActorsOfClass` "/Game/AI/AI_Ver1/BP_Monster.BP_Monster_C"))
    (for _array_element _outactors
      (if (not (`/Game/AI/AI_Ver1/BP_Monster.isDead` _array_element))
        (bind _returnvalue (`self.GetDistanceTo` _array_element))
        (if (< _returnvalue (`self.distance`))
          (set `self.Target Monster` _array_element)
          (set `self.distance` _returnvalue))))
    (`/Engine/EditorBlueprintResources/StandardMacros.IsValid` _target_monster
      (:`Is Valid`
        (`|AIMoveTo` self (0.0 0.0 0.0) _target_monster 500.0
          (:`OnSuccess`
            (set `self.IsAttack` true)))))))

(event `self.ReceiveTick`
  (params (DeltaSeconds :type "Float (single-precision)"))
  (bind _target_monster (`self.Target Monster`))
  (if (`self.IsStart`)
    (`/Engine/EditorBlueprintResources/StandardMacros.IsValid` (`self.Target Monster`)
      (:`Is Not Valid`
        (set `self.IsAttack` false)
        (set `self.distance` 10000.0)
        (bind _outactors (`GameplayStatics.GetAllActorsOfClass` "/Game/AI/AI_Ver1/BP_Monster.BP_Monster_C"))
        (if (> (`KismetArrayLibrary.Array_Length` _outactors) 0)
          (for _array_element _outactors
            (if (not (`/Game/AI/AI_Ver1/BP_Monster.isDead` _array_element))
              (bind _returnvalue (`self.GetDistanceTo` _array_element))
              (if (< _returnvalue (`self.distance`))
                (set `self.Target Monster` _array_element)
                (set `self.distance` _returnvalue))))
          (`|AIMoveTo` self (`self.K2_GetActorLocation` _target_monster) _target_monster 500.0
            (:`OnSuccess`
              (set `self.IsAttack` true))))))))

(event `ShotArrow`
  (`self.K2_SetActorRotation` (`KismetMathLibrary.FindLookAtRotation` (`self.K2_GetActorLocation`) (`self.K2_GetActorLocation` (`self.Target Monster`))))
  (bind _returnvalue (`|SpawnActorFromClass` "/Game/AI/AI_Ver2/BP_Arrow.BP_Arrow_C" (`SceneComponent.K2_GetComponentToWorld` (`self.Arrow1`)) "Undefined" "OverrideRootScale" null null))
  (set `/Game/AI/AI_Ver2/BP_Arrow.Target` (`self.Target Monster`) _returnvalue))

(fn `UserConstructionScript`)